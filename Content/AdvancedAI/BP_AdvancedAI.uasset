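; BP_AdvancedAI is an AI-controlled actor that runs the BT_AdvancedAI behavior tree and shows its health as debug text.
; On BeginPlay it has its AI controller start the behavior tree.
; Every Tick it draws the MHealthComponent health value, blending from green to red as health drops from its default.
; The text height comes from scaling the actor's world Z rather than adding an offset.
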(event `self.ReceiveBeginPlay`
  (`AIController.RunBehaviorTree` (`AIBlueprintHelperLibrary.GetAIController` self) "/Game/AdvancedAI/BT_AdvancedAI.BT_AdvancedAI"))

(event `self.ReceiveTick`
  (params (DeltaSeconds :type "Float (single-precision)"))
  (bind _returnvalue (`self.GetComponentByClass` "/Script/Mage.MHealthComponent"))
  (bind _health (`MHealthComponent.Health` _returnvalue))
  (bind _returnvalue_2 (/ _health (`MHealthComponent.DefaultHealth` _returnvalue)))
  (`KismetSystemLibrary.DrawDebugString` (`KismetMathLibrary.MakeVector` (.x (`self.K2_GetActorLocation`)) (.y (`self.K2_GetActorLocation`)) (* (.z (`self.K2_GetActorLocation`)) 1.6)) (`KismetStringLibrary.Conv_DoubleToString` _health) null (`KismetMathLibrary.MakeColor` (- 1.0 _returnvalue_2) _returnvalue_2 0.0)))

(fn `UserConstructionScript`)